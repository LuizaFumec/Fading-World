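; Pigeon (Pombo) Blueprint that cycles its skeletal mesh between two idle animations.
; BeginPlay starts a looping timer whose period is the sum of two idle time variables, so the first cycle begins after one full period.
; Each timer tick plays the two idles once in sequence, separated by a delay.
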(event `self.ReceiveBeginPlay`
  (`KismetSystemLibrary.K2_SetTimerDelegate` (delegate `PlayAnim`) (+ (`self.Tempo_Idle01`) (`self.Tempo_Idle02`)) true))

(event `PlayAnim`
  (`SkeletalMeshComponent.PlayAnimation` (`self.Mesh`) "/Game/Huedro_att/Pombo/Animation/Pombo_Idle.Pombo_Idle" false)
  (`KismetSystemLibrary.Delay` (`self.Tempo_Idle01`))
  (`SkeletalMeshComponent.PlayAnimation` (`self.Mesh`) "/Game/Huedro_att/Pombo/Animation/Pombo_Idle2.Pombo_Idle2" false)
  (`KismetSystemLibrary.Delay` (`self.Tempo_Idle02`)))

(fn `UserConstructionScript`)