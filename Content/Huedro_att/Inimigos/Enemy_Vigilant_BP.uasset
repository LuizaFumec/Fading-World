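; Patrolling guard enemy that chases the player on sight and sends the game to MenuMap when its box touches them.
; It loops through a Waypoints array, advancing the index SearchTime after overlapping the current waypoint.
; Every Tick, a macro tests squared distance, view angle and line trace, switching between faster chase and slower patrol.
; DebugVGL optionally draws route and sight cone; the CheckPlayerSight function duplicates the macro but is unused here.
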(event `self.ReceiveBeginPlay`
  (`AIBlueprintHelperLibrary.SimpleMoveToActor` (`self.GetController`) (`|GetArrayItem` (`self.Waypoints`))))

(event `self.CapsuleComponent.OnComponentBeginOverlap`
  (params (OverlappedComponent :type "PrimitiveComponent Object Reference") (OtherActor :type "Actor Object Reference") (OtherComp :type "PrimitiveComponent Object Reference") (OtherBodyIndex :type Integer) (bFromSweep :type Boolean) (SweepResult :type "HitResult Structure (by ref)"))
  (bind _returnvalue (+ (`self.Current_Waypoint_Index`) 1))
  (bind _aswaypoint_bp (cast `/Game/Huedro_att/Inimigos/Waypoint_BP` OtherActor))
  (if (== _aswaypoint_bp (`|GetArrayItem` (`self.Waypoints`) (`self.Current_Waypoint_Index`)))
    (`KismetSystemLibrary.Delay` (`self.SearchTime`))
    (set `self.Current_Waypoint_Index` (`KismetMathLibrary.SelectInt` _returnvalue 0 (< _returnvalue (`KismetArrayLibrary.Array_Length` (`self.Waypoints`)))))
    (`self.GoToWaypoint`)))

(event `self.ReceiveTick`
  (params (DeltaSeconds :type "Float (single-precision)"))
  (`self.DebugVGL`)
  (`self.CheckPlayerSightMacro`
    (:`PlayerSeen`
      (`AIBlueprintHelperLibrary.SimpleMoveToActor` (`self.GetController`) (`GameplayStatics.GetPlayerCharacter` 0))
      (set `CharacterMovementComponent.MaxWalkSpeed` 450.0 (`self.CharacterMovement`)))
    (:`PlayerNotSeen`
      (`self.GoToWaypoint`)
      (set `CharacterMovementComponent.MaxWalkSpeed` 250.0 (`self.CharacterMovement`)))))

(event `self.Box.OnComponentBeginOverlap`
  (params (OverlappedComponent :type "PrimitiveComponent Object Reference") (OtherActor :type "Actor Object Reference") (OtherComp :type "PrimitiveComponent Object Reference") (OtherBodyIndex :type Integer) (bFromSweep :type Boolean) (SweepResult :type "HitResult Structure (by ref)"))
  (cast `/Game/PlayerBP/Blueprints/SideScrollerCharacter` OtherActor)
  (`GameplayStatics.OpenLevel` "MenuMap"))

(fn `CheckPlayerSight`
  (returns (IsPlayerInSight :type Boolean))
  (if (<= (`self.GetSquaredDistanceTo` (`GameplayStatics.GetPlayerCharacter` 0)) (* (`self.SightDistance`) (`self.SightDistance`)))
    (if (<= (`KismetMathLibrary.DegAcos` (`KismetMathLibrary.Dot_VectorVector` (`self.GetActorForwardVector`) (`KismetMathLibrary.Normal` (- (`self.K2_GetActorLocation` (`GameplayStatics.GetPlayerCharacter` 0)) (`self.K2_GetActorLocation`))))) (`self.SightAngle`))
      (bind _outhit (`KismetSystemLibrary.LineTraceSingle` :`Start` (`self.K2_GetActorLocation`) :`End` (`self.K2_GetActorLocation` (`GameplayStatics.GetPlayerCharacter` 0)) :`TraceChannel` "TraceTypeQuery2" :`DrawDebugType` "ForOneFrame"))
      (cast `/Game/PlayerBP/Blueprints/SideScrollerCharacter` (`.HitActor` (`GameplayStatics.BreakHitResult` _outhit)))
      (return true)
      (else
        (return false)))
    (else
      (return false))))

(fn `DebugVGL`
  (bind _waypoints (`self.Waypoints`))
  (if (`self.IsDebugging`)
    (for (_array_element _array_index) (`self.Waypoints`)
      (bind (_returnvalue_x _returnvalue_y _returnvalue_z) (`KismetMathLibrary.BreakVector` (`self.K2_GetActorLocation` _array_element)))
      (bind _returnvalue (+ _array_index 1))
      (bind (_returnvalue_x_2 _returnvalue_y_2 _returnvalue_z_2) (`KismetMathLibrary.BreakVector` (`self.K2_GetActorLocation` (`|GetArrayItem` (`self.Waypoints`) (`KismetMathLibrary.SelectInt` _returnvalue 0 (< _returnvalue (`KismetArrayLibrary.Array_Length` (`self.Waypoints`))))))))
      (`KismetSystemLibrary.DrawDebugLine` (`KismetMathLibrary.MakeVector` _returnvalue_x _returnvalue_y (+ _returnvalue_z 5.0)) (`KismetMathLibrary.MakeVector` _returnvalue_x_2 _returnvalue_y_2 (+ _returnvalue_z_2 5.0)) (`self.DebugColor`) 0.0 5.0))
    (if (> (`KismetArrayLibrary.Array_Length` _waypoints) 0)
      (`KismetSystemLibrary.DrawDebugLine` (`self.K2_GetActorLocation`) (`self.K2_GetActorLocation` (`|GetArrayItem` _waypoints (`self.Current_Waypoint_Index`))) (struct :`G` 0.788541 :`B` 1.0 :`A` 1.0)))
    (`KismetSystemLibrary.DrawDebugConeInDegrees` (`self.K2_GetActorLocation`) (`self.GetActorForwardVector`) (`self.SightDistance`) (`self.SightAngle`) 45.0 12 (struct :`G` 1.0 :`B` 0.068809 :`A` 1.0) 0.0 5.0)))

(fn `GoToWaypoint`
  (`AIBlueprintHelperLibrary.SimpleMoveToActor` (`self.GetController`) (`|GetArrayItem` (`self.Waypoints`) (`self.Current_Waypoint_Index`))))

(fn `UserConstructionScript`)