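; Enemy character that patrols a looping list of waypoints and chases the player on sight, killing them on contact.
; Waypoint overlaps advance the patrol after a search delay, while a per-tick check combining distance, view angle and line trace switches between faster chase and slower patrol.
; Touching the player sets Died and calls DieFunc after a delay.
; An optional debug view draws the route and sight cone.
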(event `self.CapsuleComponent.OnComponentBeginOverlap`
  (params (OverlappedComponent :type "PrimitiveComponent Object Reference") (OtherActor :type "Actor Object Reference") (OtherComp :type "PrimitiveComponent Object Reference") (OtherBodyIndex :type Integer) (bFromSweep :type Boolean) (SweepResult :type "HitResult Structure (by ref)"))
  (bind _returnvalue (+ (`self.Current_Waypoint_Index`) 1))
  ;[1 1 1] Patrulha de Waypoint em Waypoint
  (bind _asenemy_waypoint_bp (cast `/Game/Huedro_att/Inimigos/EnemyWaypoint_BP` OtherActor))
  (if (== _asenemy_waypoint_bp (`|GetArrayItem` (`self.Waypoints`) (`self.Current_Waypoint_Index`)))
    (`KismetSystemLibrary.Delay` (`self.SearchTime`))
    (set `self.Current_Waypoint_Index` (`KismetMathLibrary.SelectInt` _returnvalue 0 (< _returnvalue (`KismetArrayLibrary.Array_Length` (`self.Waypoints`)))))
    (`self.GoToWaypoint`)))

(event `self.ReceiveBeginPlay`
  ;[1 1 1] Inicia a patrulha
  (`AIBlueprintHelperLibrary.SimpleMoveToActor` (`self.GetController`) (`|GetArrayItem` (`self.Waypoints`))))

(event `self.ReceiveTick`
  (params (DeltaSeconds :type "Float (single-precision)"))
  ;[1 1 1] Player visto e não visto / Debug
  (`self.DebugVGL`)
  (`self.CheckPlayerSight`
    (:`PlayerSeen`
      (`AIBlueprintHelperLibrary.SimpleMoveToActor` (`self.GetController`) (`GameplayStatics.GetPlayerCharacter` 0))
      (set `CharacterMovementComponent.MaxWalkSpeed` 450.0 (`self.CharacterMovement`)))
    (:`PlayerNotSeen`
      (`self.GoToWaypoint`)
      (set `CharacterMovementComponent.MaxWalkSpeed` 250.0 (`self.CharacterMovement`)))))

(event `self.CollisionBox_EnemyF.OnComponentBeginOverlap`
  (params (OverlappedComponent :type "PrimitiveComponent Object Reference") (OtherActor :type "Actor Object Reference") (OtherComp :type "PrimitiveComponent Object Reference") (OtherBodyIndex :type Integer) (bFromSweep :type Boolean) (SweepResult :type "HitResult Structure (by ref)"))
  ;[1 1 1] Colisão com Player
  (bind _asside_scroller_character (cast `/Game/PlayerBP/Blueprints/SideScrollerCharacter` OtherActor))
  (set `/Game/PlayerBP/Blueprints/SideScrollerCharacter.Died` true _asside_scroller_character)
  (`KismetSystemLibrary.Delay` 1.0)
  (`/Game/PlayerBP/Blueprints/SideScrollerCharacter.DieFunc` _asside_scroller_character))

(fn `DebugVGL`
  (bind _waypoints (`self.Waypoints`))
  (if (`self.IsDebugging`)
    (for (_array_element _array_index) (`self.Waypoints`)
      (bind (_returnvalue_x _returnvalue_y _returnvalue_z) (`KismetMathLibrary.BreakVector` (`self.K2_GetActorLocation` _array_element)))
      (bind _returnvalue (+ _array_index 1))
      (bind (_returnvalue_x_2 _returnvalue_y_2 _returnvalue_z_2) (`KismetMathLibrary.BreakVector` (`self.K2_GetActorLocation` (`|GetArrayItem` (`self.Waypoints`) (`KismetMathLibrary.SelectInt` _returnvalue 0 (< _returnvalue (`KismetArrayLibrary.Array_Length` (`self.Waypoints`))))))))
      (`KismetSystemLibrary.DrawDebugLine` (`KismetMathLibrary.MakeVector` _returnvalue_x _returnvalue_y (+ _returnvalue_z 5.0)) (`KismetMathLibrary.MakeVector` _returnvalue_x_2 _returnvalue_y_2 (+ _returnvalue_z_2 5.0)) (`self.DebugColor`)))
    (if (> (`KismetArrayLibrary.Array_Length` _waypoints) 0)
      (`KismetSystemLibrary.DrawDebugLine` (`self.K2_GetActorLocation`) (`self.K2_GetActorLocation` (`|GetArrayItem` _waypoints (`self.Current_Waypoint_Index`)))))
    (`KismetSystemLibrary.DrawDebugConeInDegrees` (`self.K2_GetActorLocation`) (`self.GetActorForwardVector`) (`self.SightDistance`) (`self.SightAngle`) 45.0 12 (struct :`R` 0.201665 :`G` 1.0 :`B` 0.053917 :`A` 1.0) 0.0 5.0)))

(fn `GoToWaypoint`
  (`AIBlueprintHelperLibrary.SimpleMoveToActor` (`self.GetController`) (`|GetArrayItem` (`self.Waypoints`) (`self.Current_Waypoint_Index`))))

(fn `UserConstructionScript`
  (`parent.UserConstructionScript`))