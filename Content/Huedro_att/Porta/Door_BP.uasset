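; Garage door Blueprint that drops shut the first time the side-scroller player character enters its trigger box.
; Box overlap passes through a DoOnce, then a cast to SideScrollerCharacter, then calls the Close event.
; Close plays the Lower timeline, sped up at BeginPlay, which slides the PortaGaragem component along relative Z.
; Because DoOnce precedes the cast, any first overlapping actor uses up the trigger, even if it is not the player.
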(event `self.ReceiveBeginPlay`
  (`TimelineComponent.SetPlayRate` (`self.Lower`) 8.0))

(event `Close`
  (bind (_direction _lower_door_value) (`Timeline|Lower` :!via `PlayFromStart`)
    (:`Update`
      (`SceneComponent.K2_SetRelativeLocation` (`self.porta_garagem`) (`KismetMathLibrary.MakeVector` 0.0 0.0 (* _lower_door_value -600.0)) false false))))

(event `self.Box.OnComponentBeginOverlap`
  (params (OverlappedComponent :type "PrimitiveComponent Object Reference") (OtherActor :type "Actor Object Reference") (OtherComp :type "PrimitiveComponent Object Reference") (OtherBodyIndex :type Integer) (bFromSweep :type Boolean) (SweepResult :type "HitResult Structure (by ref)"))
  (`/Engine/EditorBlueprintResources/StandardMacros.DoOnce` false
    (:`Completed`
      (cast `/Game/PlayerBP/Blueprints/SideScrollerCharacter` OtherActor)
      (`self.Close`))))

(fn `UserConstructionScript`)