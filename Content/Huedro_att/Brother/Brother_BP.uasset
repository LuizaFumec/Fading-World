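; Brother_BP is a pawn that walks along a list of waypoint actors in order.
; A Trigger event starts it moving to the first waypoint with SimpleMoveToActor.
; When its capsule overlaps the current EnemyWaypoint_BP, it advances the index and moves to the next one, with no bounds check at the end of the list.
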(event `Trigger`
  (`AIBlueprintHelperLibrary.SimpleMoveToActor` (`self.GetController`) (`|GetArrayItem` (`self.Waypoints`))))

(event `self.CapsuleComponent.OnComponentBeginOverlap`
  (params (OverlappedComponent :type "PrimitiveComponent Object Reference") (OtherActor :type "Actor Object Reference") (OtherComp :type "PrimitiveComponent Object Reference") (OtherBodyIndex :type Integer) (bFromSweep :type Boolean) (SweepResult :type "HitResult Structure (by ref)"))
  (bind _aswaypoint_bp (cast `/Game/Huedro_att/Inimigos/EnemyWaypoint_BP` OtherActor))
  (if (== _aswaypoint_bp (`|GetArrayItem` (`self.Waypoints`) (`self.Current_Waypoint_Index`)))
    (set `self.Current_Waypoint_Index` (+ (`self.Current_Waypoint_Index`) 1))
    (`self.GoToWaypoint`)))

(fn `GoToWaypoint`
  (`AIBlueprintHelperLibrary.SimpleMoveToActor` (`self.GetController`) (`|GetArrayItem` (`self.Waypoints`) (`self.Current_Waypoint_Index`))))

(fn `UserConstructionScript`)