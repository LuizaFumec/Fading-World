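; Side-scroller camera actor that follows the player character along Y, re-fetching the reference if invalid.
; Each Tick it sets height to an offset above the character, with a minimum based on InitialZ.
; Inside a hard-coded Y range, a timeline restarted every Tick lerps the X depth to a larger value.
; Outside, a second timeline lerps X back if FinishedT is set; otherwise X resets directly to default.
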(event `self.ReceiveBeginPlay`
  (`self.K2_SetActorLocation` (`KismetMathLibrary.MakeVector` 1727.0 -410.0 (`self.initialZ`)))
  (set `self.initialZ` 420.0)
  (bind _asside_scroller_character (cast `/Game/PlayerBP/Blueprints/SideScrollerCharacter` (`GameplayStatics.GetPlayerCharacter` 0)))
  (set `self.As Side Scroller Character` _asside_scroller_character))

(event `self.ReceiveTick`
  (params (DeltaSeconds :type "Float (single-precision)"))
  (bind (_returnvalue_x _returnvalue_y _returnvalue_z) (`KismetMathLibrary.BreakVector` (`self.K2_GetActorLocation`)))
  (bind (_returnvalue_x_2 _returnvalue_y_2 _returnvalue_z_2) (`KismetMathLibrary.BreakVector` (`self.K2_GetActorLocation`)))
  (bind _initialz (`self.initialZ`))
  (bind (_returnvalue_x_3 _returnvalue_y_3 _returnvalue_z_3) (`KismetMathLibrary.BreakVector` (`self.K2_GetActorLocation` (`self.As Side Scroller Character`))))
  (bind (_returnvalue_x_4 _returnvalue_y_4) (`KismetMathLibrary.BreakVector` (`self.K2_GetActorLocation` (`self.As Side Scroller Character`))))
  (bind _returnvalue (+ _returnvalue_z_3 212.0))
  (`/Engine/EditorBlueprintResources/StandardMacros.IsValid` (`self.As Side Scroller Character`)
    (:`Is Valid`
      _)
    (:`Is Not Valid`
      (bind _asside_scroller_character (cast `/Game/PlayerBP/Blueprints/SideScrollerCharacter` (`GameplayStatics.GetPlayerCharacter` 0)))
      (set `self.As Side Scroller Character` _asside_scroller_character)))
  (if (>= _returnvalue (+ _initialz 22.0))
    (`self.K2_SetActorLocation` (`KismetMathLibrary.MakeVector` (`self.xpadrao`) _returnvalue_y_3 _returnvalue))
    (else
      (`self.K2_SetActorLocation` (`KismetMathLibrary.MakeVector` (`self.xpadrao`) _returnvalue_y_3 _initialz))))
  (if (and (<= _returnvalue_y_4 -46840.0) (>= _returnvalue_y_4 -56570.0))
    (bind (_direction _newtrack_2) (`Timeline|Timeline_0` :!via `PlayFromStart`)
      (:`Update`
        (bind (_returnvalue_x_5 _returnvalue_y_5 _returnvalue_z_4) (`KismetMathLibrary.BreakVector` (`KismetMathLibrary.VLerp` (`self.K2_GetActorLocation`) (`KismetMathLibrary.MakeVector` 2000.0 _returnvalue_y _returnvalue_z) _newtrack_2)))
        (bind _output_get (set `self.xpadrao` _returnvalue_x_5))
        (`self.K2_SetActorLocation` (`KismetMathLibrary.MakeVector` _output_get _returnvalue_y_5 _returnvalue_z_4)))
      (:`Finished`
        (set `self.xpadrao` 2000.0)
        (set `self.finishedT` true)))
    (elif (`self.finishedT`)
      (bind (_direction_2 _newtrack_2_2) (`Timeline|Timeline_1` :!via `PlayFromStart`)
        (:`Update`
          (bind (_returnvalue_x_6 _returnvalue_y_6 _returnvalue_z_5) (`KismetMathLibrary.BreakVector` (`KismetMathLibrary.VLerp` (`self.K2_GetActorLocation`) (`KismetMathLibrary.MakeVector` 1727.0 _returnvalue_y_2 _returnvalue_z_2) _newtrack_2_2)))
          (bind _output_get_2 (set `self.xpadrao` _returnvalue_x_6))
          (`self.K2_SetActorLocation` (`KismetMathLibrary.MakeVector` _output_get_2 _returnvalue_y_6 _returnvalue_z_5)))
        (:`Finished`
          (set `self.xpadrao` 1727.0)
          (set `self.finishedT` false)))
      (else
        (set `self.xpadrao` 1727.0)))))

(fn `UserConstructionScript`)