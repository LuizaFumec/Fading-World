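; Wind zone actor for the side-scroller that slows or speeds up the player character inside its box trigger.
; Entering sets a side flag from Y positions, which picks the default walk speed and OnWind state.
; Each overlapping Tick, movement axis overrides these: +1 slows and strengthens the level's first WindDirectionalSource, -1 speeds up and weakens it.
; Leaving restores walk speed and clears OnWind.
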(event `self.ReceiveBeginPlay`
  (bind _asside_scroller_character (cast `/Game/PlayerBP/Blueprints/SideScrollerCharacter` (`GameplayStatics.GetPlayerCharacter` 0)))
  (set `self.As Side Scroller Character_0` _asside_scroller_character))

(event `self.ReceiveTick`
  (params (DeltaSeconds :type "Float (single-precision)"))
  (bind _as_side_scroller_character (`self.As Side Scroller Character`))
  (bind _charactermovement (`Character.CharacterMovement` _as_side_scroller_character))
  (if (`self.overlapping`)
    (`/Engine/EditorBlueprintResources/StandardMacros.IsValid` (`self.As Side Scroller Character`)
      (:`Is Valid`
        (bind _outactors (`GameplayStatics.GetAllActorsOfClass` "/Script/Engine.WindDirectionalSource"))
        (if (`self.right`)
          (set `CharacterMovementComponent.MaxWalkSpeed` 900.0 _charactermovement)
          (set `/Game/PlayerBP/Blueprints/SideScrollerCharacter.onWind` false _as_side_scroller_character)
          (else
            (set `CharacterMovementComponent.MaxWalkSpeed` 100.0 _charactermovement)
            (set `/Game/PlayerBP/Blueprints/SideScrollerCharacter.onWind` true _as_side_scroller_character)))
        (if (== (`/Game/PlayerBP/Blueprints/SideScrollerCharacter.axis` _as_side_scroller_character) 1.0)
          (set `CharacterMovementComponent.MaxWalkSpeed` 100.0 _charactermovement)
          (set `/Game/PlayerBP/Blueprints/SideScrollerCharacter.onWind` true _as_side_scroller_character)
          (bind _component (`WindDirectionalSource.Component` (`|GetArrayItem` _outactors)))
          (`WindDirectionalSourceComponent.SetSpeed` _component 8.0)
          (`WindDirectionalSourceComponent.SetStrength` _component 3.0)
          (elif (== (`/Game/PlayerBP/Blueprints/SideScrollerCharacter.axis` _as_side_scroller_character) -1.0)
            (set `CharacterMovementComponent.MaxWalkSpeed` 900.0 _charactermovement)
            (set `/Game/PlayerBP/Blueprints/SideScrollerCharacter.onWind` false _as_side_scroller_character)
            (`WindDirectionalSourceComponent.SetStrength` _component 0.1)
            (`WindDirectionalSourceComponent.SetSpeed` _component 0.1)))))))

(event `self.Box.OnComponentBeginOverlap`
  (params (OverlappedComponent :type "PrimitiveComponent Object Reference") (OtherActor :type "Actor Object Reference") (OtherComp :type "PrimitiveComponent Object Reference") (OtherBodyIndex :type Integer) (bFromSweep :type Boolean) (SweepResult :type "HitResult Structure (by ref)"))
  (bind (_returnvalue_x _returnvalue_y) (`KismetMathLibrary.BreakVector` (`self.K2_GetActorLocation`)))
  (bind (_returnvalue_x_2 _returnvalue_y_2) (`KismetMathLibrary.BreakVector` (`self.K2_GetActorLocation` (`self.As Side Scroller Character`))))
  (bind _asside_scroller_character (cast `/Game/PlayerBP/Blueprints/SideScrollerCharacter` OtherActor))
  (bind _output_get (set `self.As Side Scroller Character` _asside_scroller_character))
  (set `self.overlapping` true)
  (if (> _returnvalue_y _returnvalue_y_2)
    (set `self.right` true)
    (else
      (set `self.right` false)
      (set `/Game/PlayerBP/Blueprints/SideScrollerCharacter.onWind` true _output_get))))

(event `self.Box.OnComponentEndOverlap`
  (params (OverlappedComponent :type "PrimitiveComponent Object Reference") (OtherActor :type "Actor Object Reference") (OtherComp :type "PrimitiveComponent Object Reference") (OtherBodyIndex :type Integer))
  (bind _asside_scroller_character (cast `/Game/PlayerBP/Blueprints/SideScrollerCharacter` OtherActor))
  (set `self.overlapping` false)
  (set `CharacterMovementComponent.MaxWalkSpeed` 400.0 (`Character.CharacterMovement` _asside_scroller_character))
  (set `/Game/PlayerBP/Blueprints/SideScrollerCharacter.onWind` false _asside_scroller_character))

(fn `UserConstructionScript`)