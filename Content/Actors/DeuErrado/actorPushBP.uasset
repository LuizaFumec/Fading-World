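; Pullable block actor for the side-scroller that the player character can grab and drag along the Y axis.
; An overlap trigger caches the character; while overlapping, Tick attaches the block when pull is pressed, turning the character toward it and setting its pulling state.
; Releasing pull detaches the block and snaps it back to a fixed X and Z, keeping Y.
; Physics-based pushing logic exists but is disconnected.
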(event `self.ReceiveTick`
  (params (DeltaSeconds :type "Float (single-precision)"))
  (bind (_returnvalue_x _returnvalue_y) (`KismetMathLibrary.BreakVector` (`self.K2_GetActorLocation`)))
  (bind (_returnvalue_x_2 _returnvalue_y_2) (`KismetMathLibrary.BreakVector` (`self.K2_GetActorLocation`)))
  (bind _as_side_scroller_character (`self.As Side Scroller Character`))
  (bind (_returnvalue_x_3 _returnvalue_y_3) (`KismetMathLibrary.BreakVector` (`self.K2_GetActorLocation` (`self.As Side Scroller Character`))))
  (if (`self.overlapping`)
    (if (`/Game/PlayerBP/Blueprints/SideScrollerCharacter.PressinPulling` _as_side_scroller_character)
      (`self.K2_AttachToActor` _as_side_scroller_character "None" "KeepWorld" "KeepWorld" "KeepWorld")
      (if (> _returnvalue_y _returnvalue_y_3)
        (set `/Game/PlayerBP/Blueprints/SideScrollerCharacter.rightSide` true _as_side_scroller_character)
        (`self.K2_SetActorRotation` _as_side_scroller_character (struct :`Yaw` 90.0) true)
        (set `/Game/PlayerBP/Blueprints/SideScrollerCharacter.isPulling` true _as_side_scroller_character)
        (else
          (set `/Game/PlayerBP/Blueprints/SideScrollerCharacter.rightSide` false _as_side_scroller_character)
          (`self.K2_SetActorRotation` _as_side_scroller_character (struct :`Yaw` -90.0) true)
          (set `/Game/PlayerBP/Blueprints/SideScrollerCharacter.isPulling` true _as_side_scroller_character)))
      (else
        (`self.K2_DetachFromActor` "KeepWorld" "KeepWorld" "KeepWorld")
        (set `/Game/PlayerBP/Blueprints/SideScrollerCharacter.isPulling` false _as_side_scroller_character)
        (`self.K2_SetActorLocationAndRotation` (`KismetMathLibrary.MakeVector` 1200.0 _returnvalue_y_2 185.0))))))

(event `self.collisior.OnComponentBeginOverlap`
  (params (OverlappedComponent :type "PrimitiveComponent Object Reference") (OtherActor :type "Actor Object Reference") (OtherComp :type "PrimitiveComponent Object Reference") (OtherBodyIndex :type Integer) (bFromSweep :type Boolean) (SweepResult :type "HitResult Structure (by ref)"))
  (set `self.overlapping` true)
  (bind _asside_scroller_character (cast `/Game/PlayerBP/Blueprints/SideScrollerCharacter` OtherActor))
  (set `self.As Side Scroller Character` _asside_scroller_character))

(event `self.collisior.OnComponentEndOverlap`
  (params (OverlappedComponent :type "PrimitiveComponent Object Reference") (OtherActor :type "Actor Object Reference") (OtherComp :type "PrimitiveComponent Object Reference") (OtherBodyIndex :type Integer))
  (set `self.overlapping` false)
  (bind _asside_scroller_character (cast `/Game/PlayerBP/Blueprints/SideScrollerCharacter` OtherActor))
  (set `/Game/PlayerBP/Blueprints/SideScrollerCharacter.isPushing` false _asside_scroller_character))

(fn `UserConstructionScript`)