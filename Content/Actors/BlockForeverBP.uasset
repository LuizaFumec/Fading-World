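; BlockForeverBP is a one-way barrier actor for a side-scroller that turns solid permanently once the character passes through it.
; Its Box records the overlapping SideScrollerCharacter, and Tick sets CanBlock while that character's Y is below the actor's.
; When overlap ends with CanBlock set, the Box switches to the BlockAllDynamic collision profile, with no path to revert.
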(event `self.ReceiveTick`
  (params (DeltaSeconds :type "Float (single-precision)"))
  (bind (_returnvalue_x _returnvalue_y) (`KismetMathLibrary.BreakVector` (`self.K2_GetActorLocation`)))
  (bind (_returnvalue_x_2 _returnvalue_y_2) (`KismetMathLibrary.BreakVector` (`self.K2_GetActorLocation` (`self.As Side Scroller Character`))))
  (if (`self.overlapping`)
    (`/Engine/EditorBlueprintResources/StandardMacros.IsValid` (`self.As Side Scroller Character`)
      (:`Is Valid`
        (if (> _returnvalue_y _returnvalue_y_2)
          (set `self.canBlock` true)
          (else
            (set `self.canBlock` false)))))))

(event `self.Box.OnComponentBeginOverlap`
  (params (OverlappedComponent :type "PrimitiveComponent Object Reference") (OtherActor :type "Actor Object Reference") (OtherComp :type "PrimitiveComponent Object Reference") (OtherBodyIndex :type Integer) (bFromSweep :type Boolean) (SweepResult :type "HitResult Structure (by ref)"))
  (set `self.overlapping` true)
  (bind _asside_scroller_character (cast `/Game/PlayerBP/Blueprints/SideScrollerCharacter` OtherActor))
  (set `self.As Side Scroller Character` _asside_scroller_character))

(event `self.Box.OnComponentEndOverlap`
  (params (OverlappedComponent :type "PrimitiveComponent Object Reference") (OtherActor :type "Actor Object Reference") (OtherComp :type "PrimitiveComponent Object Reference") (OtherBodyIndex :type Integer))
  (set `self.overlapping` false)
  (if (`self.canBlock`)
    (`PrimitiveComponent.SetCollisionProfileName` (`self.Box`) "BlockAllDynamic" true)))

(fn `UserConstructionScript`)